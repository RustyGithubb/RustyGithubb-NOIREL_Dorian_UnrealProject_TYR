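; BP_Player is a player Blueprint that provides an orbit-style camera rotation through a SpringArm, with no movement logic.
; Despite their names, the MoveForward and MoveRight axes adjust the arm's world pitch and yaw, scaled by MouseSensi.
; Roll is held at zero and pitch is not explicitly clamped.
; BeginPlay shows the mouse cursor, and Tick does no meaningful work.
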(event EventTick
  (params (DeltaSeconds :type Float%20%28single-precision%29))
  ;[0.04371 0 1] Event Tick
  (Variables|Default|SetDelta%20Seconds DeltaSeconds))

(event EventBeginPlay
  (Variables|/Script/Engine.PlayerController|SetbShowMouseCursor (Game|GetPlayerController 0) true))

(event Input|AxisEvents|InputAxisMoveForward
  (params (AxisValue :type Float%20%28single-precision%29))
  (bind _springarm (Variables|Default|GetSpringArm))
  (bind _returnvalue (Transformation|GetWorldRotation _springarm))
  ;[0 0.1363 1] Rotation Camera
  (Transformation|SetWorldRotation _springarm (Math|Rotator|MakeRotator 0.0 (+ (.pitch _returnvalue) (* AxisValue (Variables|Default|GetMouseSensi))) (.yaw _returnvalue)) false false))

(event Input|AxisEvents|InputAxisMoveRight
  (params (AxisValue :type Float%20%28single-precision%29))
  (bind _springarm (Variables|Default|GetSpringArm))
  (bind _returnvalue (Transformation|GetWorldRotation _springarm))
  ;[0 0.1363 1] Rotation Camera
  (Transformation|SetWorldRotation _springarm (Math|Rotator|MakeRotator 0.0 (.pitch _returnvalue) (+ (.yaw _returnvalue) (* AxisValue (Variables|Default|GetMouseSensi)))) false false))

(fn ConstructionScript)