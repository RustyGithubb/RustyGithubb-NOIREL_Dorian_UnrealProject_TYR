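; Boat-mounted turret actor that aims with the player camera.
; Each tick it snaps to the boat's Turret1 or Turret2 mount, chosen by the Second flag.
; While CanControl is set, turret yaw and canon pitch ease toward the first BP_Camera's spring arm using plain FInterpTo, without angle wrapping.
; Otherwise, its Cube component copies the boat's rotation.
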(event EventBeginPlay
  ;[1 0 0] Camera
  (bind _outactors (Actor|GetAllActorsOfClass "/Game/Blueprint/BP_Camera.BP_Camera_C"))
  (bind _asbp_camera (Utilities|Casting|CastToBP_Camera (Utilities|Array|Get(acopy) _outactors)))
  (Variables|Default|SetAs%20BP%20Camera _asbp_camera))

(event EventTick
  (params (DeltaSeconds :type Float%20%28single-precision%29))
  (bind _canon (Variables|Default|GetCanon))
  (bind _boat (Variables|Default|GetBoat))
  (bind _turret (Variables|Default|GetTurret))
  (bind _returnvalue (Transformation|GetWorldRotation _canon))
  (bind _returnvalue_2 (Transformation|GetWorldRotation _turret))
  (Utilities|FlowControl|Sequence
    (:then_0
      ;[1 0 0.2153] Location
      (if (Variables|Default|GetSecond?)
        (Transformation|SetActorLocation (Transformation|GetWorldLocation (Variables|/Game/Blueprint/BP_Boat.BP_Boat_C|GetTurret1 _boat)) false false)
        (else
          (Transformation|SetActorLocation (Transformation|GetWorldLocation (Variables|/Game/Blueprint/BP_Boat.BP_Boat_C|GetTurret2 _boat)) false false)))
      (if (Variables|Default|GetCanControl)
        (Transformation|SetWorldRotation _turret (Math|Rotator|MakeRotator (.roll _returnvalue_2) (.pitch _returnvalue_2) (Math|Interpolation|FInterpTo (.yaw _returnvalue_2) (.yaw (Transformation|GetWorldRotation (Variables|/Game/Blueprint/BP_Camera.BP_Camera_C|GetSpringArm (Variables|Default|GetAs%20BP%20Camera)))) DeltaSeconds 1.0)) false false)
        (Transformation|SetWorldRotation _canon (Math|Rotator|MakeRotator (.roll _returnvalue) (Math|Interpolation|FInterpTo (.pitch _returnvalue) (.pitch (Transformation|GetWorldRotation (Variables|/Game/Blueprint/BP_Camera.BP_Camera_C|GetSpringArm (Variables|Default|GetAs%20BP%20Camera)))) DeltaSeconds 1.0) (.yaw _returnvalue)) false false)
        (else
          (Transformation|SetWorldRotation (Variables|Default|GetCube) (Transformation|GetActorRotation _boat) false false))))))

(fn ConstructionScript)