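; BP_IA is a kamikaze enemy, moved through CharacterMovement, that homes in on the first BP_Boat in the level.
; Every Tick it sets velocity and rotation toward the boat using interpolation, cruising level when far and diving faster in full 3D within range.
; A capsule hit on the boat subtracts Health; hitting either the boat or a BP_Bullet spawns an explosion and destroys the actor.
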(event OnComponentHit(CapsuleComponent)
  (params (HitComponent :type Primitive%20Component%20Object%20Reference) (OtherActor :type Actor%20Object%20Reference) (OtherComp :type Primitive%20Component%20Object%20Reference) (NormalImpulse :type Vector :default "0, 0, 0") (Hit :type Hit%20Result%20Structure%20%28by%20ref%29))
  (bind _asbp_boat (Utilities|Casting|CastToBP_Boat OtherActor)
    (:then
      (Variables|/Game/Blueprint/BP_Boat.BP_Boat_C|Sethealth _asbp_boat (- (Variables|/Game/Blueprint/BP_Boat.BP_Boat_C|Gethealth _asbp_boat) 5.0)))
    (:CastFailed
      (Utilities|Casting|CastToBP_Bullet OtherActor)))
  (Effects|SpawnEmitteratLocation "/Game/StarterContent/Particles/P_Explosion.P_Explosion" (Transformation|GetWorldLocation HitComponent) "0, 0, 0" "8.000000,8.000000,8.000000")
  (Actor|DestroyActor))

(event EventTick
  (params (DeltaSeconds :type Float%20%28single-precision%29))
  (bind _outactors (Actor|GetAllActorsOfClass "/Game/Blueprint/BP_Boat.BP_Boat_C"))
  (bind _asbp_boat (Utilities|Casting|CastToBP_Boat (Utilities|Array|Get(acopy) _outactors)))
  (if (< (Math|Vector|Distance(Vector) (Transformation|GetActorLocation _asbp_boat) (Transformation|GetActorLocation)) 1e+04)
    ;[1 1 1] Move
    (bind _outactors_2 (Actor|GetAllActorsOfClass "/Game/Blueprint/BP_Boat.BP_Boat_C"))
    (bind _asbp_boat_2 (Utilities|Casting|CastToBP_Boat (Utilities|Array|Get(acopy) _outactors_2)))
    (Variables|/Script/Engine.MovementComponent|SetVelocity (Variables|Character|GetCharacterMovement) (* (Math|Interpolation|VInterpTo (Math|Vector|GetForwardVector (Transformation|GetActorRotation)) (* (Math|Vector|GetUnitDirection(Vector) (Transformation|GetActorLocation) (Transformation|GetWorldLocation (Variables|/Game/Blueprint/BP_Boat.BP_Boat_C|GetBoat _asbp_boat_2))) 1e+01) DeltaSeconds 1e+01) 8e+02))
    (Transformation|SetActorRotation (Math|Interpolation|RInterpTo (Transformation|GetActorRotation) (Math|Conversions|RotationFromXVector (* (Math|Vector|GetUnitDirection(Vector) (Transformation|GetActorLocation) (Transformation|GetWorldLocation (Variables|/Game/Blueprint/BP_Boat.BP_Boat_C|GetBoat _asbp_boat_2))) 1e+01)) DeltaSeconds 1e+02))
    (else
      ;[1 1 1] Move
      (bind _outactors_3 (Actor|GetAllActorsOfClass "/Game/Blueprint/BP_Boat.BP_Boat_C"))
      (bind _asbp_boat_3 (Utilities|Casting|CastToBP_Boat (Utilities|Array|Get(acopy) _outactors_3)))
      (Variables|/Script/Engine.MovementComponent|SetVelocity (Variables|Character|GetCharacterMovement) (Math|Vector|MakeVector (.x (* (Math|Interpolation|VInterpTo (Math|Vector|GetForwardVector (Transformation|GetActorRotation)) (* (Math|Vector|GetUnitDirection(Vector) (Transformation|GetActorLocation) (Transformation|GetWorldLocation (Variables|/Game/Blueprint/BP_Boat.BP_Boat_C|GetBoat _asbp_boat_3))) 1e+01) DeltaSeconds 1e+01) 3e+02)) (.y (* (Math|Interpolation|VInterpTo (Math|Vector|GetForwardVector (Transformation|GetActorRotation)) (* (Math|Vector|GetUnitDirection(Vector) (Transformation|GetActorLocation) (Transformation|GetWorldLocation (Variables|/Game/Blueprint/BP_Boat.BP_Boat_C|GetBoat _asbp_boat_3))) 1e+01) DeltaSeconds 1e+01) 3e+02)) 0.0))
      (Transformation|SetActorRotation (Math|Rotator|MakeRotator (.roll (Math|Interpolation|RInterpTo (Transformation|GetActorRotation) (Math|Conversions|RotationFromXVector (* (Math|Vector|GetUnitDirection(Vector) (Transformation|GetActorLocation) (Transformation|GetWorldLocation (Variables|/Game/Blueprint/BP_Boat.BP_Boat_C|GetBoat _asbp_boat_3))) 1e+01)) DeltaSeconds 1e+02)) 0.0 (.yaw (Math|Interpolation|RInterpTo (Transformation|GetActorRotation) (Math|Conversions|RotationFromXVector (* (Math|Vector|GetUnitDirection(Vector) (Transformation|GetActorLocation) (Transformation|GetWorldLocation (Variables|/Game/Blueprint/BP_Boat.BP_Boat_C|GetBoat _asbp_boat_3))) 1e+01)) DeltaSeconds 1e+02)))))))

(fn ConstructionScript)