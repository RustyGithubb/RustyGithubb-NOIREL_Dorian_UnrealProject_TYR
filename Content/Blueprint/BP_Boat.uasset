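; Player-driven boat pawn with a turret, camera control, UI widget and health that triggers a return to the menu.
; Held inputs open Tick-polled gates that build persistent throttle and rudder values, driving movement, yaw and camera rotation.
; Shoot launches physics bullets from the target turret; SwitchPawn cycles a three-way selection on BP_ControllerGlobal.
; Tick also runs a countdown that periodically spawns BP_IA actors at randomized, elevated locations.
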(event Custom|CameraRotateControl
  (bind _rotateforce (Variables|Default|GetRotateForce))
  (bind _rotaterightvalue (Variables|Default|GetRotateRightValue))
  (bind _rotateforwardvalue (Variables|Default|GetRotateForwardValue))
  (bind _cam (Variables|Default|GetCam))
  (bind _returnvalue (Transformation|GetActorRotation _cam))
  (bind _returnvalue_2 (Transformation|GetActorRotation _cam))
  (bind _returnvalue_3 (+ (.yaw _returnvalue_2) _rotaterightvalue))
  (bind _returnvalue_4 (+ (.pitch _returnvalue_2) _rotateforwardvalue))
  (bind _returnvalue_5 (* _returnvalue_3 _rotateforce))
  (bind _returnvalue_6 (* _returnvalue_4 _rotateforce))
  (bind _returnvalue_7 (Math|Rotator|Lerp(Rotator) _returnvalue (Math|Rotator|MakeRotator (.roll _returnvalue_2) _returnvalue_6 _returnvalue_5) 1.0))
  ;[1 0 0.1678] RotateControl
  (Transformation|SetActorRotation _cam (Math|Rotator|MakeRotator (+ (.roll _returnvalue_7) 0.0) (+ (.pitch _returnvalue_7) 0.0) (+ (.yaw _returnvalue_7) (* (Variables|Default|GetScale%20Value%20Right) (* (Variables|Default|GetGouvernailForce) 1.0))))))

(event EventBeginPlay
  (bind _returnvalue (UserInterface|CreateWidget "/Game/Blueprint/UI.UI_C" (Game|GetPlayerController 0)))
  (UserInterface|Viewport|AddtoViewport _returnvalue 0))

(event EventTick
  (params (DeltaSeconds :type Float%20%28single-precision%29))
  (bind _returnvalue (Transformation|GetActorLocation))
  (Utilities|FlowControl|Sequence
    (:then_0
      ;[0.08991 0 1] GearsUP
      (Utilities|FlowControl|Gate true
        (:Exit
          (Variables|Default|SetScale%20Value%20Forward (+ (Variables|Default|GetScale%20Value%20Forward) (Utilities|Time|GetWorldDeltaSeconds))))))
    (:then_1
      (Utilities|FlowControl|Gate true
        (:Exit
          (Variables|Default|SetScale%20Value%20Forward (- (Variables|Default|GetScale%20Value%20Forward) (Utilities|Time|GetWorldDeltaSeconds))))))
    (:then_2
      ;[1 0 0.02677] MoveControl
      (Pawn|Input|AddMovementInput (Math|Vector|GetForwardVector (Variables|Default|GetBoat)) (* (Variables|Default|GetScale%20Value%20Forward) (Variables|Default|GetMoveForce)) false))
    (:then_3
      (Pawn|Input|AddControllerYawInput (* (* (Variables|Default|GetScale%20Value%20Right) (Variables|Default|GetGouvernailForce)) 1.0)))
    (:then_4
      ;[1 0 0.4326] Gouvernail
      (Utilities|FlowControl|Gate true
        (:Exit
          (Variables|Default|SetScale%20Value%20Right (+ (Variables|Default|GetScale%20Value%20Right) (Utilities|Time|GetWorldDeltaSeconds))))))
    (:then_5
      (Utilities|FlowControl|Gate true
        (:Exit
          (Variables|Default|SetScale%20Value%20Right (- (Variables|Default|GetScale%20Value%20Right) (Utilities|Time|GetWorldDeltaSeconds))))))
    (:then_6
      (CallFunction|CameraRotateControl))
    (:then_7
      (if (<= (- (Variables|Default|Geti) DeltaSeconds) 0.0)
        (for _index (range 0 (Variables|Default|GetLast%20Index))
          (Game|SpawnActorfromClass "/Game/Blueprint/BP_IA.BP_IA_C" (Math|Transform|MakeTransform (Math|Vector|MakeVector (* (.x _returnvalue) (Math|Random|RandomFloatinRange -2e+01 2e+01)) (* (.y _returnvalue) (Math|Random|RandomFloatinRange -2e+01 2e+01)) 5e+03) "0, 0, 0" "1,1,1") "Undefined" 0 0))
        (Variables|Default|Seti 1e+01)
        (else
          (Variables|Default|Seti (- (Variables|Default|Geti) DeltaSeconds)))))
    (:then_8
      (if (< (Variables|Default|Gethealth) 0.0)
        (Actor|DestroyActor)
        (Utilities|FlowControl|Delay 2.0)
        (Game|OpenLevel(byName) "LVL_Menu")))))

(event Input|ActionEvents|InputActionMoveUp
  (params (Key :type Key%20Structure :default "None"))
  ;[0.08991 0 1] GearsUP
  (:Pressed
    (Utilities|FlowControl|Gate true) ; enters at Open
  )
  (:Released
    (Utilities|FlowControl|Gate true) ; enters at Close
  ))

(event Input|ActionEvents|InputActionMoveDown
  (params (Key :type Key%20Structure :default "None"))
  ;[0.08991 0 1] GearsUP
  (:Pressed
    (Utilities|FlowControl|Gate true) ; enters at Open
  )
  (:Released
    (Utilities|FlowControl|Gate true) ; enters at Close
  ))

(event Input|ActionEvents|InputActionMoveRight
  (params (Key :type Key%20Structure :default "None"))
  ;[1 0 0.4326] Gouvernail
  (:Pressed
    (Utilities|FlowControl|Gate true) ; enters at Open
  )
  (:Released
    (Utilities|FlowControl|Gate true) ; enters at Close
  ))

(event Input|ActionEvents|InputActionMoveLeft
  (params (Key :type Key%20Structure :default "None"))
  ;[1 0 0.4326] Gouvernail
  (:Pressed
    (Utilities|FlowControl|Gate true) ; enters at Open
  )
  (:Released
    (Utilities|FlowControl|Gate true) ; enters at Close
  ))

(event Input|ActionEvents|InputActionSwitchPawn
  (params (Key :type Key%20Structure :default "None"))
  (:Pressed
    (bind _outactors (Actor|GetAllActorsOfClass "/Game/Blueprint/BP_ControllerGlobal.BP_ControllerGlobal_C"))
    (bind _asbp_controller_global (Utilities|Casting|CastToBP_ControllerGlobal (Utilities|Array|Get(acopy) _outactors)))
    (if (>= (+ (Variables|/Game/Blueprint/BP_ControllerGlobal.BP_ControllerGlobal_C|GetSelection _asbp_controller_global) 1) 3)
      (Variables|/Game/Blueprint/BP_ControllerGlobal.BP_ControllerGlobal_C|SetSelection _asbp_controller_global 0)
      (else
        (Variables|/Game/Blueprint/BP_ControllerGlobal.BP_ControllerGlobal_C|SetSelection _asbp_controller_global (+ (Variables|/Game/Blueprint/BP_ControllerGlobal.BP_ControllerGlobal_C|GetSelection _asbp_controller_global) 1))))))

(event Input|ActionEvents|InputActionShoot
  (params (Key :type Key%20Structure :default "None"))
  (:Pressed
    (bind _asbp_turret_actor (Utilities|Casting|CastToBP_TurretActor (Variables|Default|GetTarget)))
    (bind _returnvalue (Game|SpawnActorfromClass "/Game/Blueprint/BP_Bullet.BP_Bullet_C" (Math|Transform|MakeTransform (Transformation|GetWorldLocation (Variables|/Game/Blueprint/BP_TurretActor.BP_TurretActor_C|GetBulletSpawn _asbp_turret_actor)) (Transformation|GetWorldRotation (Variables|/Game/Blueprint/BP_TurretActor.BP_TurretActor_C|GetBulletSpawn _asbp_turret_actor)) "1,1,1") "Undefined" 0 0))
    (Physics|AddForce (Variables|/Game/Blueprint/BP_Bullet.BP_Bullet_C|GetSphere _returnvalue) (* (Math|Vector|GetForwardVector (Variables|/Game/Blueprint/BP_TurretActor.BP_TurretActor_C|GetCanon _asbp_turret_actor)) (Variables|Default|GetForce)) "None" false)))

(event Input|AxisEvents|InputAxisRotateForward
  (params (AxisValue :type Float%20%28single-precision%29))
  ;[1 0 0.1678] RotateControl
  (Variables|Default|SetRotateForwardValue AxisValue))

(event Input|AxisEvents|InputAxisRotateRight
  (params (AxisValue :type Float%20%28single-precision%29))
  ;[1 0 0.1678] RotateControl
  (Variables|Default|SetRotateRightValue AxisValue))

(fn ConstructionScript)