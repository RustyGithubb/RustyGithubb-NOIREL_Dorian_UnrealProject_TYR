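; BP_ControllerGlobal switches camera focus and control between the boat and two turrets according to a Selection value.
; BeginPlay caches the first BP_Boat, its Sphere component and the first two BP_TurretActors found.
; Each Tick re-finds BP_Camera, retargets it, eases its spring-arm length closer for turrets and toggles each turret's CanControl.
; Only the first turret's case sets the boat's Target; the second turret's equivalent is unwired.
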(event EventBeginPlay
  ;[1 0 0.03225] Cam
  ;;[0 1 0.866] Reference
  (bind _outactors (Actor|GetAllActorsOfClass "/Game/Blueprint/BP_Boat.BP_Boat_C"))
  (bind _asbp_boat (Utilities|Casting|CastToBP_Boat (Utilities|Array|Get(acopy) _outactors)))
  (Variables|Default|SetAs%20BP%20Boat_0 _asbp_boat)
  (Variables|Default|SetCube (Variables|/Game/Blueprint/BP_Boat.BP_Boat_C|GetSphere _asbp_boat))
  (bind _outactors_2 (Actor|GetAllActorsOfClass "/Game/Blueprint/BP_TurretActor.BP_TurretActor_C"))
  (Variables|Default|SetAs%20BP%20Turret1 (Utilities|Array|Get(acopy) _outactors_2))
  (bind _outactors_3 (Actor|GetAllActorsOfClass "/Game/Blueprint/BP_TurretActor.BP_TurretActor_C"))
  (Variables|Default|SetAs%20BP%20Turret2 (Utilities|Array|Get(acopy) _outactors_3 1)))

(event EventTick
  (params (DeltaSeconds :type Float%20%28single-precision%29))
  ;[1 0 0.03225] Cam
  (switch int (Variables|Default|GetSelection)
    (:0
      ;;[0 0.1965 1] Boat
      (bind _outactors (Actor|GetAllActorsOfClass "/Game/Blueprint/BP_Camera.BP_Camera_C"))
      (bind _asbp_camera (Utilities|Casting|CastToBP_Camera (Utilities|Array|Get(acopy) _outactors)))
      (Variables|/Game/Blueprint/BP_Camera.BP_Camera_C|SetTargetComp _asbp_camera (Variables|Default|GetCube))
      (Game|Player|SetViewTargetwithBlend (Game|GetPlayerController 0) _asbp_camera 0.0 "VTBlend_Linear" 0.0 false)
      (Variables|/Script/Engine.SpringArmComponent|SetTargetArmLength (Variables|/Game/Blueprint/BP_Camera.BP_Camera_C|GetSpringArm _asbp_camera) (Math|Interpolation|FInterpTo (Variables|/Script/Engine.SpringArmComponent|GetTargetArmLength (Variables|/Game/Blueprint/BP_Camera.BP_Camera_C|GetSpringArm _asbp_camera)) 1e+03 DeltaSeconds 2.0))
      (bind _asbp_turret_actor (Utilities|Casting|CastToBP_TurretActor (Variables|Default|GetAs%20BP%20Turret2)))
      (Variables|/Game/Blueprint/BP_TurretActor.BP_TurretActor_C|SetCanControl _asbp_turret_actor false)
      (bind _asbp_turret_actor_2 (Utilities|Casting|CastToBP_TurretActor (Variables|Default|GetAs%20BP%20Turret1)))
      (Variables|/Game/Blueprint/BP_TurretActor.BP_TurretActor_C|SetCanControl _asbp_turret_actor_2 false))
    (:1
      ;;[1 0 0] Turret
      (bind _outactors_2 (Actor|GetAllActorsOfClass "/Game/Blueprint/BP_Camera.BP_Camera_C"))
      (bind _asbp_camera_2 (Utilities|Casting|CastToBP_Camera (Utilities|Array|Get(acopy) _outactors_2)))
      (bind _asbp_turret_actor_3 (Utilities|Casting|CastToBP_TurretActor (Variables|Default|GetAs%20BP%20Turret1)))
      (Variables|/Game/Blueprint/BP_Camera.BP_Camera_C|SetTargetComp _asbp_camera_2 (Variables|/Game/Blueprint/BP_TurretActor.BP_TurretActor_C|GetCameraPos _asbp_turret_actor_3))
      (Variables|/Game/Blueprint/BP_TurretActor.BP_TurretActor_C|SetCanControl _asbp_turret_actor_3 true)
      (Variables|/Script/Engine.SpringArmComponent|SetTargetArmLength (Variables|/Game/Blueprint/BP_Camera.BP_Camera_C|GetSpringArm _asbp_camera_2) (Math|Interpolation|FInterpTo (Variables|/Script/Engine.SpringArmComponent|GetTargetArmLength (Variables|/Game/Blueprint/BP_Camera.BP_Camera_C|GetSpringArm _asbp_camera_2)) 1e+02 DeltaSeconds 2.0))
      (Development|PrintString "1")
      (bind _asbp_turret_actor_4 (Utilities|Casting|CastToBP_TurretActor (Variables|Default|GetAs%20BP%20Turret2)))
      (Variables|/Game/Blueprint/BP_TurretActor.BP_TurretActor_C|SetCanControl _asbp_turret_actor_4 false)
      (Variables|/Game/Blueprint/BP_Boat.BP_Boat_C|SetTarget (Variables|Default|GetAs%20BP%20Boat_0) (Variables|Default|GetAs%20BP%20Turret1)))
    (:2
      (bind _outactors_3 (Actor|GetAllActorsOfClass "/Game/Blueprint/BP_Camera.BP_Camera_C"))
      (bind _asbp_camera_3 (Utilities|Casting|CastToBP_Camera (Utilities|Array|Get(acopy) _outactors_3)))
      (bind _asbp_turret_actor_5 (Utilities|Casting|CastToBP_TurretActor (Variables|Default|GetAs%20BP%20Turret2)))
      (Variables|/Game/Blueprint/BP_Camera.BP_Camera_C|SetTargetComp _asbp_camera_3 (Variables|/Game/Blueprint/BP_TurretActor.BP_TurretActor_C|GetCameraPos _asbp_turret_actor_5))
      (Variables|/Game/Blueprint/BP_TurretActor.BP_TurretActor_C|SetCanControl _asbp_turret_actor_5 true)
      (Variables|/Script/Engine.SpringArmComponent|SetTargetArmLength (Variables|/Game/Blueprint/BP_Camera.BP_Camera_C|GetSpringArm _asbp_camera_3) (Math|Interpolation|FInterpTo (Variables|/Script/Engine.SpringArmComponent|GetTargetArmLength (Variables|/Game/Blueprint/BP_Camera.BP_Camera_C|GetSpringArm _asbp_camera_3)) 1e+02 DeltaSeconds 2.0))
      (Development|PrintString "2")
      (bind _asbp_turret_actor_6 (Utilities|Casting|CastToBP_TurretActor (Variables|Default|GetAs%20BP%20Turret1)))
      (Variables|/Game/Blueprint/BP_TurretActor.BP_TurretActor_C|SetCanControl _asbp_turret_actor_6 false))))

(fn ConstructionScript)